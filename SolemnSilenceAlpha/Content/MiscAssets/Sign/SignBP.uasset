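; Sign Blueprint with point lights that show which doors in the level have been unlocked.
; On BeginPlay it binds handlers to unlock dispatchers on the G door, P door, C door valve, C door pipe and O door lever references.
; Each handler turns the matching point light green, with both C door sources driving the same light and the O door driving the E light.
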(event Custom|G_light
  (params (G_Door :type BP%20Door%20Object%20Reference))
  (Rendering|Components|Light|SetLightColor (Variables|Default|GetG_PointLight) "(R=0.000000,G=1.000000,B=0.058809,A=1.000000)" true))

(event Custom|O_light
  (params (O_Door :type BP%20Leverinvisible%201%20Object%20Reference))
  (Rendering|Components|Light|SetLightColor (Variables|Default|GetE_PointLight) "(R=0.000000,G=1.000000,B=0.058809,A=1.000000)" true))

(event Custom|P_light
  (params (P_Door :type Pipe%20Room%20Door%20Object%20Reference))
  (Rendering|Components|Light|SetLightColor (Variables|Default|GetP_PointLight) "(R=0.000000,G=1.000000,B=0.058809,A=1.000000)" true))

(event Custom|C_light
  (params (C_Door :type BP%20Valve%20Object%20Reference))
  (Rendering|Components|Light|SetLightColor (Variables|Default|GetC_PointLight) "(R=0.000000,G=1.000000,B=0.058809,A=1.000000)" true))

(event Custom|cLight
  (params (c_door :type BP%20Pipe%20Object%20Reference))
  (Rendering|Components|Light|SetLightColor (Variables|Default|GetC_PointLight) "(R=0.000000,G=1.000000,B=0.058809,A=1.000000)" true))

(event EventBeginPlay
  (EventDispatchers|BindEventtoGDoorUnlocked (Variables|Default|GetG_Door) (delegate Custom|G_light))
  (EventDispatchers|BindEventtoPDoorUnlocked (Variables|Default|GetP_Door) (delegate Custom|P_light))
  (EventDispatchers|BindEventtoCDoorUnlocked (Variables|Default|GetC_Door_Valve) (delegate Custom|C_light))
  (EventDispatchers|BindEventtoCDoorUnlocked (Variables|Default|GetC_Door_Pipe) (delegate Custom|cLight))
  (EventDispatchers|BindEventtoOutDoorUnlocked (Variables|Default|GetO_Door_Lever) (delegate Custom|O_light)))

(fn ConstructionScript)